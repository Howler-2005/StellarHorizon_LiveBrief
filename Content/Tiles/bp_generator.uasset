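; Tile grid generator actor that spawns a Bp_tile for each row and column of a configurable grid.
; GenerateTiles clears previous tiles, spawns each new one at the generator's transform with its row and column, then calls its StartUp with Egrid.
; Spawned tiles are kept in an array that ClearOldTiles destroys and empties.
; BeginPlay and the construction script are empty, so generation is not triggered within this Blueprint.
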(fn `clear old tiles`
  (bind _tiles (`self.tiles`))
  (if (> (`KismetArrayLibrary.Array_Length` (`self.tiles`)) 0)
    (bind (_arrayindex _arrayelement) (`/Engine/EditorBlueprintResources/StandardMacros.ReverseForEachLoop` _tiles)
      (:`LoopBody`
        (`self.K2_DestroyActor` _arrayelement))
      (:`Completed`
        (`KismetArrayLibrary.Array_Clear` _tiles)))))

(fn `generate tiles`
  (`self.clear old tiles`)
  (for _index (range (`self.rows`))
    (for _index_2 (range (`self.collomes`))
      (bind _returnvalue (`|SpawnActorFromClass` "/Game/Tiles/bp_tile.bp_tile_C" (`KismetMathLibrary.MakeTransform` (`self.K2_GetActorLocation`) (`self.K2_GetActorRotation`)) "AlwaysSpawn" "MultiplyWithRoot" self _index _index_2 null))
      (`/Game/Tiles/bp_tile.start up` _returnvalue (`self.Egrid`))
      (`KismetArrayLibrary.Array_Add` (`self.tiles`) _returnvalue))))

(fn `UserConstructionScript`)