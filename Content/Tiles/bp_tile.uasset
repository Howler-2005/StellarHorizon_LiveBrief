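; A grid tile actor that displays a coloured plane and can show a selected or default highlight.
; StartUp sets the mesh for the tile type, attaches the tile to its owner, and offsets it by row and column using its mesh bounds.
; Setting the mesh also creates a dynamic instance of M_tiles, whose colour parameter OnInteract switches for selection, returning whether that material was valid.
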(event `self.ReceiveBeginPlay`
  (`self.setmesh` "NewEnumerator0"))

(fn `changeMaterial`
  (bind _returnvalue (`PrimitiveComponent.CreateDynamicMaterialInstance` (`self.tile`) 0 "/Game/Tiles/materials/tiles/m_tiles.m_tiles" "None"))
  (bind _output_get (set `self.Mat` _returnvalue))
  (`MaterialInstanceDynamic.SetVectorParameterValue` _output_get "colour" (`self.Defualtcolour`)))

(fn `OnInteract`
  (params (selected :type Boolean))
  (returns (ReturnSelected :type Boolean))
  (locals (NewLocalVar :type "MaterialInstanceDynamic Object Reference"))
  (bind _mat (`self.Mat`)
    (:`then`
      (`MaterialInstanceDynamic.SetVectorParameterValue` _mat "colour" (`KismetMathLibrary.SelectColor` (`self.selectedcolour`) (`self.Defualtcolour`) (`local.selected`)))
      (return true))
    (:`else`
      (return false))))

(fn `setmesh`
  (params (`in Grid` :type "/Game/Tiles/Egrid Enum" :default "NewEnumerator0"))
  (`StaticMeshComponent.SetStaticMesh` (`self.tile`) (select `/Game/Tiles/Egrid` `in Grid` :`NewEnumerator0` "/Game/StarterContent/Shapes/Shape_Plane.Shape_Plane" :!type "StaticMesh Object Reference"))
  (`self.changeMaterial`))

(fn `start up`
  (params (`tile type` :type "/Game/Tiles/Egrid Enum" :default "NewEnumerator0"))
  (bind _returnvalue (`self.GetOwner`))
  (`/Engine/EditorBlueprintResources/StandardMacros.IsValid` _returnvalue
    (:`Is Valid`
      (`self.setmesh` `tile type`)
      (`self.K2_AttachToActor` _returnvalue "None" "SnapToTarget" "SnapToTarget" "KeepRelative" false)
      (`self.K2_SetActorRelativeLocation` (`KismetMathLibrary.MakeVector` (* (.x (`.BoxExtent` (`KismetSystemLibrary.GetComponentBounds` (`self.tile`)))) (`self.collume`) 2.0) (* (.y (`.BoxExtent` (`KismetSystemLibrary.GetComponentBounds` (`self.tile`)))) (`self.row`) 2.0))))))

(fn `UserConstructionScript`)