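; BP_TutBot is a tutorial bot NPC that shows its dialogue lines to the player one at a time.
; Each Talk event advances TalkIndex and writes that Dialogue entry into a WBP_Dialogue widget, which is created and added to the viewport if none is valid.
; Once the index passes the last line, the widget is removed from the screen, and the index is never reset here.
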(event `/Game/TutorialBot/BPI_Dialogue.Talk`
  ;[1 1 1] NPC Dialogue
  (`/Engine/EditorBlueprintResources/StandardMacros.IncrementInt` (`self.Talk Index`)
    (:`  `
      (if (< (`self.Talk Index`) (`KismetArrayLibrary.Array_Length` (`self.Dialogue`)))
        (`self.UI`
          (:`then`
            _)
          (:`else`
            (bind _returnvalue (`|CreateWidget` "/Game/TutorialBot/WBP_Dialogue.WBP_Dialogue_C" (`GameplayStatics.GetPlayerController` 0)))
            (bind _output_get (set `self.UI` _returnvalue))
            (`UserWidget.AddToViewport` _output_get 0)))
        (`TextBlock.SetText` (`/Game/TutorialBot/WBP_Dialogue.TutBot_Dialogue` (`self.UI`)) (`KismetTextLibrary.Conv_StringToText` (`|GetArrayItem` (`self.Dialogue`) (`self.Talk Index`))))
        (else
          (`Widget.RemoveFromParent` (`self.UI`)))))))

(fn `UserConstructionScript`)